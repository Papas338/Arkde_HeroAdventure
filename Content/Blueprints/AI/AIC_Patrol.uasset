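; AI controller for a patrolling character that turns perception of player-type HA_Characters into Blackboard state.
; On perception updates it reads stimuli by array index: sight sets bIsSeeingPlayer, damage sets bHasReceivedDamage and, if receiving damage, TargetLocation.
; The BT_Patrol launch with its WaitingTime setup and an older duplicate perception handler are unwired, so this graph never starts the behavior tree.
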(event `self.ReceiveBeginPlay`)

(event `self.AIPerception.OnPerceptionUpdated`
  (params (UpdatedActors :type "Array of Actor Object Reference (by ref)"))
  (bind _breceivingdamage (`self.bReceivingDamage`))
  (for _array_element UpdatedActors
    (bind _info (`AIPerceptionComponent.GetActorsPerception` (`self.AIPerceptionComponent`) _array_element))
    (bind _asha_character (cast `HA_Character` (break `ActorPerceptionBlueprintInfo` _info)))
    (bind _returnvalue (`HA_Character.GetCharacterType` _asha_character))
    (if (`|EnumEquality` _returnvalue "CharacterType_Player")
      (for (_array_element_2 _array_index) (`.LastSensedStimuli` (break `ActorPerceptionBlueprintInfo` _info))
        (switch `int` _array_index
          (:`0`
            ;[1 1 1] Sight
            (`BlackboardComponent.SetValueAsBool` (`AIBlueprintHelperLibrary.GetBlackboard` null) "bIsSeeingPlayer" (`.bSuccessfullySensed` (break `AIStimulus` _array_element_2))))
          (:`1`
            ;[1 1 1] Damage
            (`KismetSystemLibrary.PrintString` "Damage")
            (`BlackboardComponent.SetValueAsBool` (`AIBlueprintHelperLibrary.GetBlackboard` null) "bHasReceivedDamage" _breceivingdamage)
            (if _breceivingdamage
              (`BlackboardComponent.SetValueAsVector` (`AIBlueprintHelperLibrary.GetBlackboard` null) "TargetLocation" (`.StimulusLocation` (break `AIStimulus` _array_element_2))))))))))

(fn `UserConstructionScript`)