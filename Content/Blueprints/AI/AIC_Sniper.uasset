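; AI controller for the sniper enemy that reports whether it currently senses the player.
; On each perception update it filters the updated actors for player-type HA_Character targets.
; The first sensed stimulus's success state is written to the bIsSeeingPlayer Blackboard key.
; Nodes that would run BT_Sniper and set WaitingTime are disconnected, so this graph never starts the behavior tree.
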(event `self.ReceiveBeginPlay`)

(event `self.AIPerception.OnPerceptionUpdated`
  (params (UpdatedActors :type "Array of Actor Object Reference (by ref)"))
  (for _array_element UpdatedActors
    (bind _info (`AIPerceptionComponent.GetActorsPerception` (`self.AIPerceptionComponent`) _array_element))
    (bind _asha_character (cast `HA_Character` (break `ActorPerceptionBlueprintInfo` _info)))
    (bind _returnvalue (`HA_Character.GetCharacterType` _asha_character))
    (if (`|EnumEquality` _returnvalue "CharacterType_Player")
      (for (_array_element_2 _array_index) (`.LastSensedStimuli` (break `ActorPerceptionBlueprintInfo` _info))
        (switch `int` _array_index
          (:`0`
            (`|ExecutionSequence`
              (:`then_0`
                (`BlackboardComponent.SetValueAsBool` (`AIBlueprintHelperLibrary.GetBlackboard` null) "bIsSeeingPlayer" (`.bSuccessfullySensed` (break `AIStimulus` _array_element_2)))))))))))

(fn `UserConstructionScript`)