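; BP_Character is a character Blueprint that sets up the main HUD and changes screen post-processing while the ultimate ability is usable.
; BeginPlay adds W_MainHUD to the viewport and caches the PostProcess component's settings as NormalPostProcess.
; Tick polls GetCanUseUltimate every frame and assigns either UltimateReadyPostProcess or the cached settings, with no state-change check.
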(event `self.ReceiveBeginPlay`
  (`|ExecutionSequence`
    (:`then_0`
      (bind _returnvalue (`|CreateWidget` "/Game/Blueprints/UI/HUD/W_MainHUD.W_MainHUD_C"))
      (`UserWidget.AddToViewport` _returnvalue 0))
    (:`then_1`
      (set `self.NormalPostProcess` (`PostProcessComponent.Settings` (`self.PostProcess`))))))

(event `self.ReceiveTick`
  (params (DeltaSeconds :type "Float (single-precision)"))
  (bind _returnvalue (`self.GetCanUseUltimate`))
  (if _returnvalue
    (set `PostProcessComponent.Settings` (`self.UltimateReadyPostProcess`) (`self.PostProcess`))
    (else
      (set `PostProcessComponent.Settings` (`self.NormalPostProcess`) (`self.PostProcess`)))))

(fn `UserConstructionScript`)